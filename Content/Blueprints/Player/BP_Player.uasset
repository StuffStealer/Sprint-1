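; BP_Player is the player Blueprint, where collected coins add life and taking damage removes life and spawns coins around the player.
; Attack rises or falls in steps whenever life lands on a multiple of five, and is exposed through a getter.
; BeginPlay creates the HUD widget, which receives the updated stats struct after each change.
; Tick prints the attack value for debugging.
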(event `self.ReceiveTick`
  (params (DeltaSeconds :type "Float (single-precision)"))
  (`KismetSystemLibrary.Delay` 0.5)
  (`KismetSystemLibrary.PrintString` (`KismetStringLibrary.Concat_StrStr` "DAMAGE : " (`KismetStringLibrary.Conv_DoubleToString` (`.Attack_16_334E2A3746BF3B0169F161846A582E16` (break `/Game/Blueprints/Player/Struct_Player_Stats` (`self.Struct_Player`))))) true true (struct :`R` 1.0 :`B` 0.1103 :`A` 1.0) 0.5))

(event `Key|C`
  (params (Key :type "Key Structure")))

(event `self.ReceiveBeginPlay`
  (`self.Setup_Player`))

(event `/Game/Blueprints/Player/BPI_Player.BF_Add_Coins`
  (bind ((`Current_Life_13_2EADDF0A4226669FD14AD39A509D5794` _current_life) (`Attack_16_334E2A3746BF3B0169F161846A582E16` _attack)) (break `/Game/Blueprints/Player/Struct_Player_Stats` (`self.Struct_Player`)))
  (bind _result (`/Engine/EditorBlueprintResources/StandardMacros.IncrementInt` _current_life)
    (:`  `
      (if (not (`KismetMathLibrary.Conv_IntToBool` (mod _result 5)))
        (setmembers `/Game/Blueprints/Player/Struct_Player_Stats` :`StructRef` (`self.Struct_Player`) :`Attack` (+ _attack 10.0)))
      (set `/Game/Blueprints/Player/Widget/WIB_HUD.struct_Player` (`self.Struct_Player`) (`self.Ref_WIB_HUD`)))))

(event `self.ReceiveAnyDamage`
  (params (Damage :type "Float (single-precision)") (DamageType :type "DamageType Object Reference") (InstigatedBy :type "Controller Object Reference") (DamageCauser :type "Actor Object Reference"))
  (bind (_max_life _current_life _attack) (break `/Game/Blueprints/Player/Struct_Player_Stats` (`self.Struct_Player`)))
  (bind _returnvalue (`KismetMathLibrary.Clamp` (`KismetMathLibrary.FTrunc` (- _current_life Damage)) 0 _max_life))
  (setmembers `/Game/Blueprints/Player/Struct_Player_Stats` :`StructRef` (`self.Struct_Player`) :`Current_Life` _returnvalue)
  (if (not (`KismetMathLibrary.Conv_IntToBool` (mod _returnvalue 5)))
    (setmembers `/Game/Blueprints/Player/Struct_Player_Stats` :`StructRef` (`self.Struct_Player`) :`Attack` (`KismetMathLibrary.FClamp` (- _attack 10.0) 0.0 100.0)))
  (set `/Game/Blueprints/Player/Widget/WIB_HUD.struct_Player` (`self.Struct_Player`) (`self.Ref_WIB_HUD`))
  (`self.Spawn_Coins`))

(event `Spawn_Coins`
  (bind _returnvalue (`SceneComponent.K2_GetComponentLocation` (`self.Mesh`)))
  (`|SpawnActorFromClass` "/Game/Blueprints/Colectible/Childs/BP_CC_Coins.BP_CC_Coins_C" (`KismetMathLibrary.MakeTransform` (`KismetMathLibrary.MakeVector` (.x (+ _returnvalue (* (`KismetMathLibrary.RotateAngleAxis` _returnvalue (`KismetMathLibrary.RandomFloatInRange` 0.0 360.0) (* (`KismetMathLibrary.Vector_Up`) 0.2)) 0.1))) (.y (+ _returnvalue (* (`KismetMathLibrary.RotateAngleAxis` _returnvalue (`KismetMathLibrary.RandomFloatInRange` 0.0 360.0) (* (`KismetMathLibrary.Vector_Up`) 0.2)) 0.1))) 0.5)) "Undefined" "MultiplyWithRoot" null null))

(fn `BF_Attack_Set`
  (returns (Attack :type "Float (double-precision)"))
  (return (`.Attack_16_334E2A3746BF3B0169F161846A582E16` (break `/Game/Blueprints/Player/Struct_Player_Stats` (`self.Struct_Player`)))))

(fn `Setup_Player`
  (bind _returnvalue (`|CreateWidget` "/Game/Blueprints/Player/Widget/WIB_HUD.WIB_HUD_C" null (`self.Struct_Player`)))
  (bind _output_get (set `self.Ref_WIB_HUD` _returnvalue))
  (`UserWidget.AddToViewport` _output_get 0)
  (`WidgetBlueprintLibrary.SetInputMode_GameOnly` (`GameplayStatics.GetPlayerController` 0))
  (set `PlayerController.bShowMouseCursor` false (`GameplayStatics.GetPlayerController` 0)))

(fn `UserConstructionScript`)