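; Trader Blueprint for a shop-style interaction with hat and sunglasses cosmetics, currently inactive: InteractMenu and ResetPlayer are empty and both logic chains are unconnected.
; The unconnected open chain shows the trader widget, toggles movement, blends the view and caches the player's hat and glasses meshes.
; The unconnected close chain removes the widget, restores game input and camera, and reapplies the cached meshes.
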(event `/Game/Blueprints/Trader/BPI_Trader.Interact_Menu`)

(event `/Game/Blueprints/Trader/BPI_Trader.Reset_Player`)

(fn `UserConstructionScript`)