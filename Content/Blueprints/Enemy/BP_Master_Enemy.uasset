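; Master enemy Blueprint that takes damage, gains strength from coins and drops coins on death.
; A stats struct holds life, attack and coins; damage reduces clamped life, and at zero it spawns coins before destroying itself.
; The drop adds held coins to a base quantity, scattering them at randomly rotated offsets and fixed height.
; BFAddCoins raises attack every fifth coin, and BFGetAttack exposes that value.
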(event `Spawn_Coin`
  (bind _returnvalue (`self.K2_GetActorLocation`))
  (bind ((`Coins_11_B653339F440B7E8E8B56509F10C60F8B` _coins)) (break `/Game/Blueprints/Enemy/Struct_Enemy_Stats` (`self.Struct_Enemy`)))
  (if (not (== _coins 0))
    (set `self.Quantity_Coins` (+ _coins (`self.Quantity_Coins`))))
  (for _ (range (+ (`self.Quantity_Coins`) 1))
    (`|SpawnActorFromClass` "/Game/Blueprints/Colectible/Childs/BP_CC_Coins.BP_CC_Coins_C" (`KismetMathLibrary.MakeTransform` (`KismetMathLibrary.MakeVector` (.x (+ _returnvalue (* (`KismetMathLibrary.RotateAngleAxis` _returnvalue (`KismetMathLibrary.RandomFloatInRange` 0.0 360.0) (* (`KismetMathLibrary.Vector_Up`) 0.2)) 0.2))) (.y (+ _returnvalue (* (`KismetMathLibrary.RotateAngleAxis` _returnvalue (`KismetMathLibrary.RandomFloatInRange` 0.0 360.0) (* (`KismetMathLibrary.Vector_Up`) 0.2)) 0.2))) 50.0)) "Undefined" "MultiplyWithRoot" null null)))

(event `self.ReceiveAnyDamage`
  (params (Damage :type "Float (single-precision)") (DamageType :type "DamageType Object Reference") (InstigatedBy :type "Controller Object Reference") (DamageCauser :type "Actor Object Reference"))
  (bind ((`Max_Life_3_41CFDBE349BD101056B073B2879FD517` _max_life) (`Current_Life_5_D7DE60D5434024BDE06ECFB235CFCB89` _current_life)) (break `/Game/Blueprints/Enemy/Struct_Enemy_Stats` (`self.Struct_Enemy`)))
  (bind _returnvalue (`KismetMathLibrary.FClamp` (- _current_life Damage) 0.0 _max_life))
  (setmembers `/Game/Blueprints/Enemy/Struct_Enemy_Stats` :`StructRef` (`self.Struct_Enemy`) :`Current_Life` _returnvalue)
  (if (<= _returnvalue 0.0)
    (`self.Spawn_Coin`)
    (`self.K2_DestroyActor`)))

(event `/Game/Blueprints/Enemy/BPI_Enemy.BF_Add_Coins`
  (bind ((`Attack_8_38A4F2564DD9D6543827F7A5FAEE984D` _attack) (`Coins_11_B653339F440B7E8E8B56509F10C60F8B` _coins)) (break `/Game/Blueprints/Enemy/Struct_Enemy_Stats` (`self.Struct_Enemy`)))
  (bind _result (`/Engine/EditorBlueprintResources/StandardMacros.IncrementInt` _coins)
    (:`  `
      (if (not (`KismetMathLibrary.Conv_IntToBool` (mod _result 5)))
        (setmembers `/Game/Blueprints/Enemy/Struct_Enemy_Stats` :`StructRef` (`self.Struct_Enemy`) :`Attack` (+ _attack 5.0))))))

(fn `BF_Get_Attack`
  (returns (Attack :type "Float (double-precision)"))
  (return (`.Attack_8_38A4F2564DD9D6543827F7A5FAEE984D` (break `/Game/Blueprints/Enemy/Struct_Enemy_Stats` (`self.Struct_Enemy`)))))

(fn `UserConstructionScript`)