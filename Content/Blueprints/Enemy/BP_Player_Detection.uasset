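; BP_Player_Detection is a trigger volume that alerts a set of enemies when the player enters it.
; On Box overlap, it checks that the other actor's class is exactly BP_Player, then loops over the RefBPEnemy array.
; It sets the "Player_In_Range?" Blackboard key to true on each enemy, and nothing here clears it when the player leaves.
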(event `self.Box.OnComponentBeginOverlap`
  (params (OverlappedComponent :type "PrimitiveComponent Object Reference") (OtherActor :type "Actor Object Reference") (OtherComp :type "PrimitiveComponent Object Reference") (OtherBodyIndex :type Integer) (bFromSweep :type Boolean) (SweepResult :type "HitResult Structure (by ref)"))
  (if (and (== (`GameplayStatics.GetObjectClass` OtherActor) "/Game/Blueprints/Player/BP_Player.BP_Player_C") (`KismetArrayLibrary.Array_IsNotEmpty` (`self.Ref_BP_Enemy`)))
    (for _array_element (`self.Ref_BP_Enemy`)
      (`BlackboardComponent.SetValueAsBool` (`AIBlueprintHelperLibrary.GetBlackboard` _array_element) "Player_In_Range?" true))))

(fn `UserConstructionScript`)